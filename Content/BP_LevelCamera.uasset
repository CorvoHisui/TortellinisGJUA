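; BP_LevelCamera is a shared camera that follows two characters and zooms with their separation.
; Each tick it eases toward their midpoint plus an offset using a constant-alpha lerp.
; It likewise eases spring arm length in proportion to their distance, clamped between minimum and maximum lengths.
; The reference distance, despite being named InitialCharacterDistance, is measured at BeginPlay between the first two BP_MapEdge actors.
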(event EventBeginPlay
  (bind _outactors (Actor|GetAllActorsOfClass "/Game/BP_MapEdge.BP_MapEdge_C"))
  (Variables|Default|SetInitialCharacterDistance (Math|Vector|Distance(Vector) (Transformation|GetActorLocation (Utilities|Array|Get(acopy) _outactors)) (Transformation|GetActorLocation (Utilities|Array|Get(acopy) _outactors 1)))))

(event Collision|EventActorBeginOverlap
  (params (OtherActor :type Actor%20Object%20Reference)))

(event EventTick
  (params (DeltaSeconds :type Float%20%28single-precision%29))
  (bind _character1 (Variables|Default|GetCharacter1))
  (bind _character2 (Variables|Default|GetCharacter2))
  (bind _springarm (Variables|Default|GetSpringArm))
  (bind _returnvalue (Transformation|GetActorLocation _character2))
  (bind _returnvalue_2 (Transformation|GetActorLocation _character1))
  (Variables|Default|SetDistanceBetweenCharacters (Math|Vector|Distance(Vector) _returnvalue_2 _returnvalue))
  (Variables|Default|SetObjectiveLocation (+ (/ (- _returnvalue _returnvalue_2) 2.0) _returnvalue_2))
  (Transformation|SetActorLocation (Math|Vector|Lerp(Vector) (Transformation|GetActorLocation) (+ (Variables|Default|GetObjectiveLocation) (Variables|Default|GetCameraOffset)) 0.1) false false)
  (Variables|Default|SetObjectiveCameraLength (* (/ (Math|Float|Min(Float) (Variables|Default|GetInitialCharacterDistance) (Variables|Default|GetDistanceBetweenCharacters)) (Variables|Default|GetInitialCharacterDistance)) (Variables|Default|GetMaxCameraLength)))
  (Variables|/Script/Engine.SpringArmComponent|SetTargetArmLength _springarm (Math|Float|Clamp(Float) (Math|Float|Lerp (Variables|/Script/Engine.SpringArmComponent|GetTargetArmLength _springarm) (Variables|Default|GetObjectiveCameraLength) 0.1) (Variables|Default|GetMinCameraLength) (Variables|Default|GetMaxCameraLength))))

(fn ConstructionScript)